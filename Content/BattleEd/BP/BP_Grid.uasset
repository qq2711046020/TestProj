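; BP_Grid is a grid cell actor in the BattleEd folder, with a plane whose look can be changed at runtime.
; BeginPlay creates a dynamic material instance from the plane's material and stores it.
; SetBorder and SetColor events drive that instance's Border scalar, as an on/off switch, and its Color vector at full alpha.
; GetModuleName returns a module path matching the asset, which suggests a script binding such as UnLua.
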(event Custom|SetColor
  (params (Value%20R :type Float%20%28single-precision%29) (Value%20G :type Float%20%28single-precision%29) (Value%20B :type Float%20%28single-precision%29))
  (Rendering|Material|SetVectorParameterValue (Variables|Default|GetMI) "Color" (Utilities|Struct|MakeLinearColor Value%20R Value%20G Value%20B 1.0) :!class /Script/Engine.MaterialInstanceDynamic))

(event Custom|SetBorder
  (params (bPickA :type Boolean))
  (Rendering|Material|SetScalarParameterValue (Variables|Default|GetMI) "Border" (Math|Float|SelectFloat 1.0 0.0 bPickA) :!class /Script/Engine.MaterialInstanceDynamic))

(event EventBeginPlay
  (bind _plane (Variables|Default|GetPlane))
  (bind _returnvalue (Rendering|Material|CreateDynamicMaterialInstance _plane 0 (Rendering|Material|GetMaterial _plane 0) "None" :!class /Script/Engine.PrimitiveComponent))
  (Variables|Default|SetMI _returnvalue))

(event Collision|EventActorBeginOverlap
  (params (OtherActor :type Actor%20Object%20Reference)))

(event EventTick
  (params (DeltaSeconds :type Float%20%28single-precision%29)))

(fn ConstructionScript)

(fn GetModuleName
  (return "BattleEd.BP.BP_Grid"))